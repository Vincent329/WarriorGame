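; Base enemy character Blueprint that handles death: ragdoll, dissolve effect and cleanup.
; On death it disables capsule collision, simulates mesh physics and async-loads the supplied Niagara system, attaching it to the mesh with particles tinted from the material's dissolve edge color.
; A timeline scaled by total dissolve time then drives the dissolve parameter on body and equipped weapon materials, destroying both actors when finished.
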(event `self.ReceiveBeginPlay`)

(event `/Game/Enemies/BPI_EnemyDeath.OnEnemyDied`
  (params (DissolveNiagaraSystem :type "NiagaraSystem Soft Object Reference"))
  (bind _mesh (`self.Mesh`))
  (bind _mesh_2 (`self.Mesh`))
  (bind _returnvalue (`PawnCombatComponent.GetCharacterCurrentEquippedWeapon` (`self.EnemyCombatComponent`)))
  (bind _returnvalue_2 (`PawnCombatComponent.GetCharacterCurrentEquippedWeapon` (`self.EnemyCombatComponent`)))
  (`|ExecutionSequence`
    (:`then_0`
      (`PrimitiveComponent.SetCollisionEnabled` (`self.CapsuleComponent`) "NoCollision")
      (`PrimitiveComponent.SetCollisionProfileName` _mesh "Ragdoll" true)
      (`PrimitiveComponent.SetSimulatePhysics` _mesh true))
    (:`then_1`
      (bind _object (`|LoadAsset` DissolveNiagaraSystem)
        (:`Completed`
          ; cast will only succeed once the asset is loaded
          (bind _asniagara_system (cast `NiagaraSystem` _object))
          (bind _returnvalue_3 (`NiagaraFunctionLibrary.SpawnSystemAttached` _asniagara_system (`self.Mesh`) "None" (0.0 0.0 0.0) (struct) "KeepRelativeOffset" true))
          (bind _returnvalue_4 (`PrimitiveComponent.CreateDynamicMaterialInstance` _mesh_2 0 (`PrimitiveComponent.GetMaterial` _mesh_2 0) "None"))
          (bind _returnvalue_5 (`MaterialInstanceDynamic.K2_GetVectorParameterValue` _returnvalue_4 "DissolveEdgeColor"))
          (`NiagaraComponent.SetNiagaraVariableLinearColor` _returnvalue_3 "DissolveParticleColor" _returnvalue_5)
          (`TimelineComponent.SetPlayRate` (`self.Timeline`) (/ 1.0 (`self.Total Dissolve Time`)))
          (bind (_direction _normalized_float_dissolve_lerp_value) (`Timeline|Timeline`)
            (:`Update`
              (`MeshComponent.SetScalarParameterValueOnMaterials` (`self.Mesh`) "DissolveAmount" _normalized_float_dissolve_lerp_value)
              (`/Engine/EditorBlueprintResources/StandardMacros.IsValid` _returnvalue_2
                (:`Is Valid`
                  (`MeshComponent.SetScalarParameterValueOnMaterials` (`WarriorBaseWeapon.WeaponMesh` _returnvalue_2) "DissolveAmount" _normalized_float_dissolve_lerp_value))))
            (:`Finished`
              (`/Engine/EditorBlueprintResources/StandardMacros.IsValid` _returnvalue
                (:`Is Valid`
                  ; Think about another way to destroy... Enemy pool
                  (`self.K2_DestroyActor` _returnvalue))
                (:`Is Not Valid`
                  _))
              (`self.K2_DestroyActor`))))))))

(fn `UserConstructionScript`)