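; BP_RotatingPlatform is a platform actor that spins continuously around its vertical axis.
; Each Tick adds relative yaw to PlatformMesh, scaling RotationSpeed by DeltaSeconds so the spin is frame-rate independent.
; BeginPlay and ActorBeginOverlap are disabled stubs, and the construction script only calls its parent.
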(event `self.ReceiveTick`
  (params (DeltaSeconds :type "Float (single-precision)"))
  (`parent.ReceiveTick` DeltaSeconds)
  (`SceneComponent.K2_AddRelativeRotation` (`self.PlatformMesh`) (`KismetMathLibrary.MakeRotator` 0.0 0.0 (* DeltaSeconds (`self.Rotation Speed`))) false false))

(fn `UserConstructionScript`
  (`parent.UserConstructionScript`))