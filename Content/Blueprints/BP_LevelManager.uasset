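; BP_LevelManager is a manager actor meant to swap out randomly chosen level pieces, each represented by an actor.
; Its GenerateNewLevels event currently only destroys every actor in ActiveLevels, and BeginPlay is empty.
; An unconnected spawn loop picks random LevelArray classes and places them at the root location plus TransformMark.
; That loop never runs and neither updates the offset nor records spawned actors in ActiveLevels.
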(event `self.ReceiveBeginPlay`)

(event `GenerateN ewLevels`
  (for _array_element (`self.ActiveLevels`)
    (`self.K2_DestroyActor` _array_element)))

(fn `UserConstructionScript`)