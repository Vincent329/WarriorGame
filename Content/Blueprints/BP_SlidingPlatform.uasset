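; BP_SlidingPlatform is a platform that slides back and forth between its root location and a DestinationPoint.
; BeginPlay caches both world positions, scales the timeline rate by Duration and starts in the direction set by IsGoingForward.
; SlidingTimeline lerps PlatformMesh between them without sweeping.
; On finishing, it waits PauseTimer, flips the direction flag and plays the opposite way, looping indefinitely.
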(event `self.ReceiveBeginPlay`
  (`parent.ReceiveBeginPlay`)
  (set `self.StartPoint` (`SceneComponent.K2_GetComponentLocation` (`self.DefaultSceneRoot`)))
  (set `self.EndPoint` (`SceneComponent.K2_GetComponentLocation` (`self.DestinationPoint`)))
  (`TimelineComponent.SetPlayRate` (`self.Sliding Timeline`) (/ 1.0 (`self.Duration`)))
  (if (`self.IsGoingForward`)
    (`self.Start Forward`)
    (else
      (`self.Start Backward`))))

(event `Forward`
  (bind (_direction _newtrack_0) (`Timeline|Sliding Timeline` :!label _label)
    (:`Update`
      (`SceneComponent.K2_SetWorldLocation` (`self.PlatformMesh`) (`KismetMathLibrary.VLerp` (`self.StartPoint`) (`self.EndPoint`) _newtrack_0) false false))
    (:`Finished`
      (`KismetSystemLibrary.Delay` (`self.PauseTimer`))
      (if (`self.IsGoingForward`)
        (set `self.IsGoingForward` false)
        (`self.Backward`)
        (else
          (set `self.IsGoingForward` true)
          (`self.Forward`))))))

(event `Start Forward`
  (goto _label :!via `PlayFromStart`))

(event `Backward`
  (goto _label :!via `Reverse`))

(event `Start Backward`
  (goto _label :!via `ReverseFromEnd`))

(fn `UserConstructionScript`
  (`parent.UserConstructionScript`))